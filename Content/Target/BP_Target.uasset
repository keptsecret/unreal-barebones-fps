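; BP_Target is a shootable target actor that awards score to whoever hits it and reports itself to the game mode.
; On BeginPlay it records starting health, creates a dynamic material from M_Target and messages the game mode that a target was added.
; Each hit awards score, subtracts damage and lerps the color from green toward red by remaining health.
; At zero health it grants a bonus, notifies the game mode and destroys itself.
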(event EventHandleWasHit
  (params (Hitter :type Actor%20Object%20Reference) (DmgValue :type Integer))
  (Variables|Default|SetHitter Hitter)
  (Variables|Default|SetDmg%20Value DmgValue)
  (Class|FPSControllerBPI|HandleUpdateScore(Message) (Variables|Default|GetHitter) (Variables|Config|GetTargetValue))
  (Variables|Config|SetHealthValue (- (Variables|Config|GetHealthValue) (Variables|Default|GetDmg%20Value)))
  (CallFunction|SetColor)
  (if (<= (Variables|Config|GetHealthValue) 0)
    (Class|FPSControllerBPI|HandleUpdateScore(Message) (Variables|Default|GetHitter) (Variables|Default|GetBonusValue))
    (Class|FPSGameModeBPI|RemoveTarget(Message) (Game|GetGameMode))
    (Actor|DestroyActor)))

(event EventBeginPlay
  (Variables|Default|SetStartingHealthValue (Variables|Config|GetHealthValue))
  (bind _returnvalue (Rendering|Material|CreateDynamicMaterialInstance "/Game/Materials/M_Target.M_Target" "None" "None" :!class /Script/Engine.KismetMaterialLibrary))
  (bind _output_get (Variables|Default|SetDynamicMat _returnvalue))
  (Rendering|Material|SetMaterial (Variables|Default|GetCube) 0 _output_get)
  (CallFunction|SetColor)
  (Class|FPSGameModeBPI|AddTarget(Message) (Game|GetGameMode)))

(fn ConstructionScript)

(fn SetColor
  (Rendering|Material|SetVectorParameterValue (Variables|Default|GetDynamicMat) "Color" (Math|Color|Lerp(LinearColor) "(R=1.000000,G=0.000000,B=0.000000,A=1.000000)" "(R=0.000000,G=1.000000,B=0.000000,A=1.000000)" (/ (Math|Conversions|ToFloat(Integer) (Variables|Config|GetHealthValue)) (Math|Conversions|ToFloat(Integer) (Variables|Default|GetStartingHealthValue)))) :!class /Script/Engine.MaterialInstanceDynamic))